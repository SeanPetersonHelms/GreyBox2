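; Game instance Blueprint that provides shared helper functions for starting music and showing the player HUD and game over screen.
; Start Music creates and plays a 2D sound at a given volume, stores it as Audio, and can keep it playing across level transitions.
; The two UI functions each create a widget owned by the first player controller and add it to the viewport.
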(fn StartMusic
  (params (Audio :type Sound%20Base%20Object%20Reference) (Volume :type Float%20%28single-precision%29) (Persist? :type Boolean))
  (bind _returnvalue (Audio|CreateSound2D Audio Volume 1.0 0.0 0 Persist?))
  (bind _output_get (Variables|Default|SetAudio _returnvalue))
  (Audio|Components|Audio|Play _output_get 0.0))

(fn MakePlayerHUD
  (bind _returnvalue (UserInterface|CreateWidget "/Game/Menus/Widgets/HUD.HUD_C" (Class|GameplayStatics|GetPlayerControllerfromID)))
  (UserInterface|Viewport|AddtoViewport _returnvalue 0))

(fn MakeGameOverScreen
  (bind _returnvalue (UserInterface|CreateWidget "/Game/Menus/Widgets/PlayerDeath.PlayerDeath_C" (Class|GameplayStatics|GetPlayerControllerfromID)))
  (UserInterface|Viewport|AddtoViewport _returnvalue 0))